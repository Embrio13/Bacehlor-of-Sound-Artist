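; BP_DualAutoDoor is an automatic double sliding door that opens for the first-person character.
; Begin overlap on PlayerDetection plays the DoorOpen timeline and end overlap reverses it, both filtered by a FirstPersonCharacter cast.
; The timeline track slides DoorRight and DoorLeft in opposite directions along relative X.
; Each update overwrites both full relative transforms, with DoorRight mirrored through fixed rotation and negative scale.
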(event OnComponentBeginOverlap(PlayerDetection)
  (params (OverlappedComponent :type Primitive%20Component%20Object%20Reference) (OtherActor :type Actor%20Object%20Reference) (OtherComp :type Primitive%20Component%20Object%20Reference) (OtherBodyIndex :type Integer) (bFromSweep :type Boolean) (SweepResult :type Hit%20Result%20Structure%20%28by%20ref%29))
  (Utilities|Casting|CastToFirstPersonCharacter OtherActor)
  (bind _newtrack_0 (Timeline|DoorOpen Play)
    (:Update
      (Transformation|SetRelativeTransform (Variables|Default|GetDoorRight) (Math|Transform|MakeTransform (Math|Vector|MakeVector _newtrack_0 0.0 0.0) "0,0.000000,180.000000" "-1.000000,-1.000000,-1.000000") false false)
      (Transformation|SetRelativeTransform (Variables|Default|GetDoorLeft) (Math|Transform|MakeTransform (Math|Vector|MakeVector (* _newtrack_0 -1.0) 0.0 0.0) "0,0.000000, 0") false false))))

(event OnComponentEndOverlap(PlayerDetection)
  (params (OverlappedComponent :type Primitive%20Component%20Object%20Reference) (OtherActor :type Actor%20Object%20Reference) (OtherComp :type Primitive%20Component%20Object%20Reference) (OtherBodyIndex :type Integer))
  (Utilities|Casting|CastToFirstPersonCharacter OtherActor)
  (bind _newtrack_0 (Timeline|DoorOpen Reverse)
    (:Update
      (Transformation|SetRelativeTransform (Variables|Default|GetDoorRight) (Math|Transform|MakeTransform (Math|Vector|MakeVector _newtrack_0 0.0 0.0) "0,0.000000,180.000000" "-1.000000,-1.000000,-1.000000") false false)
      (Transformation|SetRelativeTransform (Variables|Default|GetDoorLeft) (Math|Transform|MakeTransform (Math|Vector|MakeVector (* _newtrack_0 -1.0) 0.0 0.0) "0,0.000000, 0") false false))))

(event EventBeginPlay)

(event Collision|EventActorBeginOverlap
  (params (OtherActor :type Actor%20Object%20Reference)))

(event EventTick
  (params (DeltaSeconds :type Float%20%28single-precision%29)))

(fn ConstructionScript)