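; BP_AutoDoor is an automatic door that opens when the first-person character enters its PlayerDetection volume.
; Entry posts a Wwise door sound and debug print, then plays the DoorOpen timeline, which drives the Door's relative Z.
; Exit reverses the timeline without sound.
; The opening sits behind a DoOnce with no reset, so later entries replay only the sound and print.
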(event OnComponentBeginOverlap(PlayerDetection)
  (params (OverlappedComponent :type Primitive%20Component%20Object%20Reference) (OtherActor :type Actor%20Object%20Reference) (OtherComp :type Primitive%20Component%20Object%20Reference) (OtherBodyIndex :type Integer) (bFromSweep :type Boolean) (SweepResult :type Hit%20Result%20Structure%20%28by%20ref%29))
  (Utilities|Casting|CastToFirstPersonCharacter OtherActor)
  (Utilities|FlowControl|Sequence
    (:then_0
      (Class|AkGameplayStatics|PostEventatLocation "/Game/WwiseAudio/Events/Default_Work_Unit/Effects/Play_doors.Play_doors" (Transformation|GetActorLocation) "0, 0, 0")
      (Development|PrintString "Hello"))
    (:then_1
      (Utilities|FlowControl|DoOnce false
        (:Completed
          (bind _newtrack_0 (Timeline|DoorOpen PlayFromStart)
            (:Update
              (Transformation|SetRelativeTransform (Variables|Default|GetDoor) (Math|Transform|MakeTransform (Math|Vector|MakeVector 5e+01 0.0 _newtrack_0)) false false))))))))

(event OnComponentEndOverlap(PlayerDetection)
  (params (OverlappedComponent :type Primitive%20Component%20Object%20Reference) (OtherActor :type Actor%20Object%20Reference) (OtherComp :type Primitive%20Component%20Object%20Reference) (OtherBodyIndex :type Integer))
  (Utilities|Casting|CastToFirstPersonCharacter OtherActor)
  (bind _newtrack_0 (Timeline|DoorOpen Reverse)
    (:Update
      (Transformation|SetRelativeTransform (Variables|Default|GetDoor) (Math|Transform|MakeTransform (Math|Vector|MakeVector 5e+01 0.0 _newtrack_0)) false false))))

(event EventBeginPlay)

(event Collision|EventActorBeginOverlap
  (params (OtherActor :type Actor%20Object%20Reference)))

(event EventTick
  (params (DeltaSeconds :type Float%20%28single-precision%29)))

(fn ConstructionScript)